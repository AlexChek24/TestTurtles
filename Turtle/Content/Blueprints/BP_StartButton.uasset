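; BP_StartButton is a mesh-based button actor that shows a text label on the HUD while the cursor hovers over it.
; On cursor over, it casts the first player controller's HUD to TurtleHud, passes in its TextName and turns on IsShow.
; On cursor exit, it turns IsShow off.
; It contains no click handling, so only the hover feedback is implemented here.
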(event OnBeginCursorOver(StaticMesh)
  (params (TouchedComponent :type Primitive%20Component%20Object%20Reference))
  (bind _asturtle_hud (Utilities|Casting|CastToTurtleHud (HUD|GetHUD (Game|GetPlayerController 0))))
  (Variables|/Game/Blueprints/TurtleHud.TurtleHud_C|SetTextName _asturtle_hud (Variables|Default|GetTextName))
  (Variables|/Game/Blueprints/TurtleHud.TurtleHud_C|SetIsShow _asturtle_hud true))

(event OnEndCursorOver(StaticMesh)
  (params (TouchedComponent :type Primitive%20Component%20Object%20Reference))
  (bind _asturtle_hud (Utilities|Casting|CastToTurtleHud (HUD|GetHUD (Game|GetPlayerController 0))))
  (Variables|/Game/Blueprints/TurtleHud.TurtleHud_C|SetIsShow _asturtle_hud false))

(event EventBeginPlay)

(event Collision|EventActorBeginOverlap
  (params (OtherActor :type Actor%20Object%20Reference)))

(event EventTick
  (params (DeltaSeconds :type Float%20%28single-precision%29)))

(fn ConstructionScript)