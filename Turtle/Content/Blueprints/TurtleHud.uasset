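; TurtleHud is a HUD Blueprint that shows a left-mouse-button prompt with a text label while IsShow is set.
; DrawHUD caches the screen size each frame, then calls ShowName when the flag is on.
; ShowName draws the key icon near the bottom, a quarter of the way across, and prints TextName in black beside it, offset by the icon's size.
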(event EventBeginPlay)

(event Collision|EventActorBeginOverlap
  (params (OtherActor :type Actor%20Object%20Reference)))

(event EventTick
  (params (DeltaSeconds :type Float%20%28single-precision%29)))

(event EventDrawHUD
  (params (SizeX :type Integer) (SizeY :type Integer))
  (Variables|Default|SetScreenSize (Math|Vector2D|MakeVector2D (Math|Conversions|ToFloat(Integer) SizeX) (Math|Conversions|ToFloat(Integer) SizeY)))
  (if (Variables|Default|GetIsShow)
    (CallFunction|ShowName)))

(fn ConstructionScript)

(fn ShowName
  (bind _screensize (Variables|Default|GetScreenSize))
  (bind (_x _y) (Math|Vector2D|BreakVector2D _screensize))
  (bind _returnvalue (/ _x 4.0))
  (bind _returnvalue_2 (- _y 1e+02))
  (bind _output_get (Variables|Default|SetIcon "/Game/KeyBoard/Mouse_Left_Key_Dark.Mouse_Left_Key_Dark"))
  (Class|HUD|DrawTextureSimple _output_get _returnvalue _returnvalue_2 1.0 false)
  (HUD|DrawText (Utilities|String|ToString(Text) (Variables|Default|GetTextName)) "(R=0.000000,G=0.000000,B=0.000000,A=1.000000)" (+ _returnvalue (Math|Conversions|ToFloat(Integer) (Class|Texture2D|BlueprintGetSizeX _output_get))) (+ _returnvalue_2 (Math|Conversions|ToFloat(Integer) (/ (Class|Texture2D|BlueprintGetSizeY _output_get) 6))) "/Game/Blueprints/times_new_roman_Font.times_new_roman_Font" 1.0 false))